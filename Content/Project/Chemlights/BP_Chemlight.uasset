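; Grabbable chemlight that glows when shaken and gradually reveals paintings near it.
; Each tick, mesh velocity or a debug toggle sets the shaken state on the luminance capacity component, held briefly after motion stops by an extension timer.
; That component's intensity percentage drives the point light's brightness.
; A sphere trace at the actor raises a hit BP_Painting's LerpValue over time; a UV brush-reveal variant is unconnected.
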(event OnGrabbed(GrabComponent))

(event OnDropped(GrabComponent))

(event Custom|StartShakeDebug
  (Variables|Default|SetVariablePressed true))

(event Custom|StopShakeDebug
  (Variables|Default|SetVariablePressed false))

(event EventTick
  (params (DeltaSeconds :type Float%20%28single-precision%29))
  (bind _returnvalue (Transformation|GetActorLocation))
  (Utilities|FlowControl|Sequence
    (:then_0
      (Rendering|Components|Light|SetIntensity (Variables|Default|GetPointLight) (Math|Float|Lerp (Variables|Intensity|GetMinIntensity) (Variables|Intensity|GetMaxIntensity) (/ (Variables|/Script/VRProject.ChemlightLuminanceCapacity|GetCurrentIntensityPercentage (Variables|Default|GetChemlightLuminanceCapacity)) 1e+02)))
      (bind _returnvalue_2 (Physics|GetPhysicsLinearVelocity (Variables|Default|GetMesh) "None"))
      (if (or (> (Math|Vector|VectorLength _returnvalue_2) (Variables|Shake|GetShakeVelocityThreshold)) (Variables|Default|GetVariablePressed))
        (if (Variables|Shake|GetIsShaking)
          (Variables|Shake|SetShakeTimer (+ (Variables|Shake|GetShakeTimer) DeltaSeconds))
          (else
            (if (Variables|Shake|GetIsShakeExtensionStarted)
              _
              (else
                (Variables|Shake|SetShakeTimer 0.0)))
            (Variables|Shake|SetIsShaking true)
            (Variables|Shake|SetIsShakeExtensionStarted false)
            (Variables|Shake|SetShakeExtensionTimer 0.0)
            (Variables|/Script/VRProject.ChemlightLuminanceCapacity|SetIsShaken (Variables|Default|GetChemlightLuminanceCapacity) true)))
        (elif (Variables|Shake|GetIsShaking)
          (Variables|Shake|SetIsShaking false)
          (Variables|Shake|SetIsShakeExtensionStarted true)
          (Variables|Shake|SetShakeExtensionTimer 0.0)
          (elif (Variables|Shake|GetIsShakeExtensionStarted)
            (if (> (Variables|Shake|GetShakeExtensionTimer) (Variables|Shake|GetShakeExtensionDuration))
              (Variables|Shake|SetIsShakeExtensionStarted false)
              (Variables|/Script/VRProject.ChemlightLuminanceCapacity|SetIsShaken (Variables|Default|GetChemlightLuminanceCapacity) false)
              (else
                (Variables|Shake|SetShakeExtensionTimer (+ DeltaSeconds (Variables|Shake|GetShakeExtensionTimer)))
                (Variables|Shake|SetShakeTimer (+ DeltaSeconds (Variables|Shake|GetShakeTimer)))))))))
    (:then_1
      (bind _outhit (Collision|SphereTraceByChannel _returnvalue _returnvalue (Variables|Default|GetLight%20Radius) "TraceTypeQuery1" true 0 "ForOneFrame"))
      (bind _asbp_painting (Utilities|Casting|CastToBP_Painting (.hitactor _outhit)))
      (Variables|/Game/Actors/BP_Painting.BP_Painting_C|SetLerpValue _asbp_painting (Math|Float|Clamp(Float) (+ (Variables|/Game/Actors/BP_Painting.BP_Painting_C|GetLerpValue _asbp_painting) (/ (Utilities|Time|GetWorldDeltaSeconds) (Variables|Default|GetReveal%20Speed))))))))

(fn ConstructionScript)