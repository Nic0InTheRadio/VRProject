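; BP_DoorLights is a door light actor that shows painting-reveal progress for one room by switching on up to three spotlights in turn.
; On BeginPlay it binds to the painting-revealed event on VRGameMode.
; When a reveal occurs while the current room index matches its IndexRoom, it increments a counter and activates the corresponding BP_DoorSpotLight child actor.
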(event Custom|Activate%20New%20Light
  (bind _result (Math|Integer|IncrementInt (Variables|Default|GetNbLightsActivated))
    (:%20%20
      (switch int _result
        (:1
          (bind _asbp_door_spot_light (Utilities|Casting|CastToBP_DoorSpotLight (Variables|/Script/Engine.ChildActorComponent|GetChildActor (Variables|Default|GetLightActor))))
          (Default|ActivateLight _asbp_door_spot_light))
        (:2
          (bind _asbp_door_spot_light_2 (Utilities|Casting|CastToBP_DoorSpotLight (Variables|/Script/Engine.ChildActorComponent|GetChildActor (Variables|Default|GetLightActor1))))
          (Default|ActivateLight _asbp_door_spot_light_2))
        (:3
          (bind _asbp_door_spot_light_3 (Utilities|Casting|CastToBP_DoorSpotLight (Variables|/Script/Engine.ChildActorComponent|GetChildActor (Variables|Default|GetLightActor2))))
          (Default|ActivateLight _asbp_door_spot_light_3))))))

(event Custom|CheckPaintingRevealed
  (if (== (Variables|/Game/VRTemplate/Blueprints/VRGameMode.VRGameMode_C|GetIndexCurrentRoom (Variables|Default|GetVRGameMode)) (Variables|Default|GetIndexRoom))
    (CallFunction|ActivateNewLight)))

(event EventBeginPlay
  (bind _asvrgame_mode (Utilities|Casting|CastToVRGameMode (Game|GetGameMode)))
  (bind _output_get (Variables|Default|SetVRGameMode _asvrgame_mode))
  (EventDispatchers|BindEventtoPaintingRevealed _output_get (delegate Custom|CheckPaintingRevealed)))

(fn ConstructionScript)