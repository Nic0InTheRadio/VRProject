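; BP_RandomSFXGenerator is an actor that plays random sound effects from the SoundToPlay2D array at random intervals.
; Tick uses the IsWaiting flag as a gate, so only one cycle is pending at a time.
; Each cycle assigns a random sound to AudioSource, waits a random whole number of seconds between MinWait and MaxWait, plays it, then reopens the gate.
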(event EventBeginPlay)

(event Collision|EventActorBeginOverlap
  (params (OtherActor :type Actor%20Object%20Reference)))

(event EventTick
  (params (DeltaSeconds :type Float%20%28single-precision%29))
  (bind _soundtoplay2d (Variables|Default|GetSoundToPlay2D))
  (if (not (Variables|Default|GetbIsWaiting))
    (Variables|Default|SetbIsWaiting true)
    (Audio|Components|Audio|SetSound (Variables|Default|GetAudioSource) (Utilities|Array|Get(acopy) _soundtoplay2d (Math|Random|RandomIntegerinRange 0 (Utilities|Array|Length _soundtoplay2d))))
    (Utilities|FlowControl|Delay (Math|Conversions|ToFloat(Integer) (Math|Random|RandomIntegerinRange (Variables|Default|GetMinWait) (Variables|Default|GetMaxWait))))
    (Audio|Components|Audio|Play (Variables|Default|GetAudioSource) 0.0)
    (Variables|Default|SetbIsWaiting false)))

(fn ConstructionScript)