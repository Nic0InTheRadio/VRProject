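; Trigger zone actor that, on any actor overlap, either plays a montage on an assigned animated actor or plays a sound.
; Sound plays via audio components on an external source actor when localized, otherwise through its own AudioSource with the assigned sound.
; A played flag and CanSoundPlayAgain gate replays.
; Exiting BoxZone can destroy the box and stop AudioSource, and both overlaps print debug strings.
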(event OnComponentEndOverlap(BoxZone)
  (params (OverlappedComponent :type Primitive%20Component%20Object%20Reference) (OtherActor :type Actor%20Object%20Reference) (OtherComp :type Primitive%20Component%20Object%20Reference) (OtherBodyIndex :type Integer))
  (bind _boxzone (Variables|Default|GetBoxZone))
  ;[1 1 1] EndOverlap
  (Development|PrintString (Utilities|GetDisplayName (Variables|Default|GetBoxZone)))
  (Utilities|FlowControl|Sequence
    (:then_0
      ;;[1 1 1] Destroy TriggerZone Check
      (if (Variables|Tweak|GetbDestroysHitbox)
        (if (Utilities|IsValid _boxzone)
          (Components|DestroyComponent _boxzone))))
    (:then_1
      ;;[1 1 1] Stop Audio Source When Exiting TriggerZone
      (if (Variables|Tweak|GetbStopSoundWhenExiting)
        (Audio|Components|Audio|Stop (Variables|Default|GetAudioSource))))))

(event Collision|EventActorBeginOverlap
  (params (OtherActor :type Actor%20Object%20Reference))
  (bind _audiosource (Variables|Default|GetAudioSource))
  ;[1 1 1] BeginOverlap
  (Development|PrintString (Utilities|GetDisplayName (Variables|Default|GetBoxZone)))
  (if (Variables|Tweak|GetbTriggerAnimation)
    ;;[1 1 1] Play Animation
    (Animation|Montage|PlayMontage (Variables|Tweak|GetAnimatedActor) (Variables|Tweak|GetMontage%20to%20Play)
      (:OnCompleted
        (Development|PrintString "Animation Finished")))
    (else
      ;;[1 1 1] Already Playing / Localized Sound Checks
      (if (Variables|Tweak|GetbIsSoundAlreadyPlaying)
        (if (Variables|Tweak|GetbCanSoundPlayAgain)
          (if (Variables|Tweak|GetbLocalizedSound) :!label _label
            ;;[1 1 1] Play Localized Sound
            (Audio|Components|Audio|Play (Actor|GetComponentsByClass (Variables|Tweak|GetExternalAudioSourceLocation) "/Script/Engine.AudioComponent") 0.0)
            (else
              ;;[1 1 1] Play Sound2D
              (Audio|Components|Audio|SetSound _audiosource (Variables|Tweak|GetSoundToPlayLocalized))
              (Audio|Components|Audio|Play _audiosource 0.0))))
        (else
          (Variables|Tweak|SetbIsSoundAlreadyPlaying true)
          (goto _label))))))

(fn ConstructionScript)