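; Door light Blueprint that starts dark and fades its light in when activated.
; On BeginPlay it stores the PointLight component's intensity as the maximum and sets it to zero.
; ActivateLight runs a linear float tween to that stored maximum over TimeToLight seconds, applying each value as intensity.
; A SetColor event changes the light's color; despite the SpotLight name, the component driven is PointLight.
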(event Custom|ActivateLight
  (bind _value (|TweenFloat 0.0 (Variables|Default|GetMaxIntensity) (Variables|Default|GetTimeToLight) "Linear")
    (:ApplyEasing
      (Rendering|Components|Light|SetIntensity (Variables|Default|GetPointLight) _value))))

(event Custom|SetColor
  (params (NewColor :type Linear%20Color%20Structure))
  (Rendering|Components|Light|SetLightColor (Variables|Default|GetPointLight) NewColor true))

(event EventBeginPlay
  (Variables|Default|SetMaxIntensity (Variables|/Script/Engine.LightComponentBase|GetIntensity (Variables|Default|GetPointLight)))
  (Rendering|Components|Light|SetIntensity (Variables|Default|GetPointLight) 0.0))

(fn ConstructionScript)