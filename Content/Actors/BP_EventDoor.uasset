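; BP_EventDoor is a VR room door that opens for the current room and shuts behind the player.
; It opens when VRGameMode's open-door event fires and IndexDoor matches the current room index.
; A VRPawn entering its box closes it and, on the first pass only, tells the game mode to change room.
; Opened and closed events play a sound and tween the pivot's yaw with sine easing.
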(event OnComponentBeginOverlap(Box)
  (params (OverlappedComponent :type Primitive%20Component%20Object%20Reference) (OtherActor :type Actor%20Object%20Reference) (OtherComp :type Primitive%20Component%20Object%20Reference) (OtherBodyIndex :type Integer) (bFromSweep :type Boolean) (SweepResult :type Hit%20Result%20Structure%20%28by%20ref%29))
  (if (Utilities|ClassIsChildOf (Utilities|GetClass OtherActor) "/Game/VRTemplate/Blueprints/VRPawn.VRPawn_C")
    (Class|Door|CloseDoor)
    (if (not (Variables|Default|GetIsClosed))
      (Variables|Default|SetIsClosed true)
      (bind _asvrgame_mode (Utilities|Casting|CastToVRGameMode (Game|GetGameMode)))
      (Default|ChangeRoom _asvrgame_mode))))

(event Custom|OpenDoorEvent
  (if (== (Variables|Default|GetIndexDoor) (Variables|/Game/VRTemplate/Blueprints/VRGameMode.VRGameMode_C|GetIndexCurrentRoom (Variables|Default|GetVRGameMode)))
    (Class|Door|OpenDoor)))

(event EventOnDoorOpened
  (Audio|PlaySoundatLocation (Variables|Default|GetOpeningSound) (Transformation|GetActorLocation) "0, 0, 0" 1.0 1.0 0.0 0 0 0 0)
  (bind _value (|TweenFloat 0.0 -9e+01 1.0 "InOutSine")
    (:ApplyEasing
      (Transformation|SetRelativeRotation (Variables|Default|GetPivotPoint) (Math|Rotator|MakeRotator 0.0 0.0 _value) false false))))

(event EventOnDoorClosed
  (Audio|PlaySoundatLocation (Variables|Default|GetClosingSound) (Transformation|GetActorLocation) "0, 0, 0" 1.0 1.0 0.0 0 0 0 0)
  (bind _value (|TweenFloat -9e+01 0.0 1.0 "InOutSine")
    (:ApplyEasing
      (Transformation|SetRelativeRotation (Variables|Default|GetPivotPoint) (Math|Rotator|MakeRotator 0.0 0.0 _value) false false))))

(event EventBeginPlay
  (bind _asvrgame_mode (Utilities|Casting|CastToVRGameMode (Game|GetGameMode)))
  (bind _output_get (Variables|Default|SetVRGameMode _asvrgame_mode))
  (EventDispatchers|BindEventtoOpenDoorEventDispatcher _output_get (delegate Custom|OpenDoorEvent)))

(fn ConstructionScript)